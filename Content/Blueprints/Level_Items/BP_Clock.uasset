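; BP_Clock is a level clock that rotates its hour and minute hands to show the time held by BP_GM.
; It binds to the game mode's clock tick and maps Hour and Minute to hand pitch.
; Each minute-hand change plays a tick sound whose volume scales with a growing counter.
; StopTime and ResumeTime toggle both the clock and the game mode's timer, with stopping also resetting that counter.
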(event `self.ReceiveBeginPlay`
  (bind _asbp_gm (cast `/Game/Blueprints/BP_GM` (`GameplayStatics.GetGameMode`)))
  (bind _output_get (set `self.As BP GM` _asbp_gm))
  (add `/Game/Blueprints/BP_GM.ClockTick` _output_get (delegate `Tick`)))

(event `Tick`
  (bind _returnvalue (`KismetMathLibrary.MapRangeClamped` (`KismetMathLibrary.Conv_IntToDouble` (`/Game/Blueprints/BP_GM.Minute` (`self.As BP GM`))) 0.0 60.0 0.0 -360.0))
  (if (`self.bPlayTime`)
    (`SceneComponent.K2_SetRelativeRotation` (`self.Minute`) (`KismetMathLibrary.MakeRotator` 0.0 _returnvalue) false false)
    (set `self.MinuteRotation` _returnvalue)
    (`SceneComponent.K2_SetRelativeRotation` (`self.Hour`) (`KismetMathLibrary.MakeRotator` 0.0 (`KismetMathLibrary.MapRangeClamped` (`KismetMathLibrary.Conv_IntToDouble` (`/Game/Blueprints/BP_GM.Hour` (`self.As BP GM`))) 0.0 12.0 0.0 -360.0)) false false)
    (if (!= (`self.MinuteRotation`) (`self.PreMinuteRotation`))
      (bind _result (`/Engine/EditorBlueprintResources/StandardMacros.IncrementInt` (`self.TickCounter`))
        (:`  `
          (`GameplayStatics.PlaySoundAtLocation` "/Game/Sounds/SFX/clock_tick/clock_tick.clock_tick" (`self.K2_GetActorLocation`) (struct) (* _result 0.01) 1.0 0.0 null null null null)
          (set `self.PreMinuteRotation` (`self.MinuteRotation`)))))))

(event `StopTime`
  (set `/Game/Blueprints/BP_GM.bTimerOn` false (`self.As BP GM`))
  (set `self.bPlayTime` false)
  (set `self.TickCounter` 0))

(event `ResumeTime`
  (set `/Game/Blueprints/BP_GM.bTimerOn` true (`self.As BP GM`))
  (set `self.bPlayTime` true))

(fn `UserConstructionScript`)