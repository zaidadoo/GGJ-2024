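; BP_CoffeeMachine is a level item that dispenses coffee after being smashed several times.
; On BeginPlay it binds to the Smash event of the BP_PhysicsObject in its CoffeeMachine child actor.
; Each smash increments a counter and compares it to a freshly rolled random threshold.
; Passing the threshold resets the counter and spawns BP_Coffee at the machine's location, with debug prints for both outcomes.
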(event `self.ReceiveBeginPlay`
  (bind _asbp_physics_object (cast `/Game/Blueprints/Level_Items/BP_PhysicsObject` (`ChildActorComponent.ChildActor` (`self.CoffeeMachine`))))
  (add `/Game/Blueprints/Level_Items/BP_PhysicsObject.Smash` _asbp_physics_object (delegate `Smash`)))

(event `Smash`
  (bind _result (`/Engine/EditorBlueprintResources/StandardMacros.IncrementInt` (`self.SmashCounter`))
    (:`  `
      (if (> _result (`KismetMathLibrary.RandomIntegerInRange` 2 5))
        (`KismetSystemLibrary.PrintString` "Spawn Coffee" true true (struct :`R` 1.0 :`G` 0.178204 :`A` 1.0))
        (set `self.SmashCounter` 0)
        (`|SpawnActorFromClass` "/Game/Blueprints/Level_Items/BP_Coffee.BP_Coffee_C" (`KismetMathLibrary.MakeTransform` (`self.K2_GetActorLocation`)) "Undefined" "MultiplyWithRoot" null null)
        (else
          (`KismetSystemLibrary.PrintString` "CoffeeMachineSmash"))))))

(fn `UserConstructionScript`)