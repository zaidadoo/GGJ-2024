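; Level phone that rings at random, plays gibberish speech when answered and goes quiet after repeated smashing.
; A Delay on Tick periodically rolls for a ring, which teleports the child BP_PhysicsObject prop back to its starting spot.
; Interacting while not tired answers a ringing phone.
; Sound rides on the prop, whose bound Smash event stops the chatter once hits exceed a freshly rolled random threshold.
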(event `Smash`
  (if (`self.bWasTalking`)
    (bind _result (`/Engine/EditorBlueprintResources/StandardMacros.IncrementInt` (`self.SmashCounter`))
      (:`  `
        (if (> _result (`KismetMathLibrary.RandomIntegerInRange` 3 8))
          (`self.StopNoise`))))))

(event `self.ReceiveBeginPlay`
  (bind _asbp_physics_object (cast `/Game/Blueprints/Level_Items/BP_PhysicsObject` (`ChildActorComponent.ChildActor` (`self.Phone`))))
  (`SceneComponent.K2_AttachToComponent` (`self.Sound`) (`/Game/Blueprints/Level_Items/BP_PhysicsObject.Prop` _asbp_physics_object) "None" "SnapToTarget" "SnapToTarget" "SnapToTarget" true)
  (bind _asbp_physics_object_2 (cast `/Game/Blueprints/Level_Items/BP_PhysicsObject` (`ChildActorComponent.ChildActor` (`self.Phone`))))
  (set `self.Original Location` (`SceneComponent.K2_GetComponentLocation` (`/Game/Blueprints/Level_Items/BP_PhysicsObject.Prop` _asbp_physics_object_2)))
  (bind _asbp_physics_object_3 (cast `/Game/Blueprints/Level_Items/BP_PhysicsObject` (`ChildActorComponent.ChildActor` (`self.Phone`))))
  (add `/Game/Blueprints/Level_Items/BP_PhysicsObject.Smash` _asbp_physics_object_3 (delegate `Smash`)))

(event `self.ReceiveTick`
  (params (DeltaSeconds :type "Float (single-precision)"))
  (`KismetSystemLibrary.Delay` 30.0)
  (if (> (`KismetMathLibrary.RandomIntegerInRange` 0 100) 50)
    (`self.PlayRingtone`)))

(event `/Game/Blueprints/Level_Items/BP_InteractInterface.Interact`
  (params (IsTired :type Boolean) (Character :type "/Game/Blueprints/BP_MainChar Object Reference"))
  (if (not IsTired)
    (`self.PlayTalker`)))

(event `PlayRingtone`
  (bind _sound (`self.Sound`))
  (bind _asbp_physics_object (cast `/Game/Blueprints/Level_Items/BP_PhysicsObject` (`ChildActorComponent.ChildActor` (`self.Phone`))))
  (`SceneComponent.K2_SetWorldLocation` (`/Game/Blueprints/Level_Items/BP_PhysicsObject.Prop` _asbp_physics_object) (`self.Original Location`) false true)
  (set `self.bWasRinging` true)
  (`AudioComponent.SetSound` _sound "/Game/Sounds/SFX/ringtone/ringtone.ringtone")
  (`AudioComponent.Play` _sound 0.0))

(event `PlayTalker`
  (bind _sound (`self.Sound`))
  (if (`self.bWasRinging`)
    (set `self.bWasTalking` true)
    (`AudioComponent.SetSound` _sound "/Game/Sounds/SFX/gibberish/gibberish_phone.gibberish_phone")
    (`AudioComponent.Play` _sound 0.0)
    (set `self.bWasRinging` false)))

(event `StopNoise`
  (`AudioComponent.Stop` (`self.Sound`))
  (set `self.SmashCounter` 0)
  (set `self.bWasRinging` false)
  (set `self.bWasTalking` false))

(fn `UserConstructionScript`)