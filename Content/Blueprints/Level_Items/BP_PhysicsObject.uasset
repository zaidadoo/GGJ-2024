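; BP_PhysicsObject is a configurable physics prop that plays smash effects on hard impacts.
; The construction script applies the chosen mesh and mass override to the Prop component.
; Hits above an impulse threshold spawn a sound and particle system picked by ImpactNoise (Fart or Metal), call the Smash dispatcher and print the force.
; A Gate closes briefly after each smash to debounce repeated hits.
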(event `self.Prop.OnComponentHit`
  (params (HitComponent :type "PrimitiveComponent Object Reference") (OtherActor :type "Actor Object Reference") (OtherComp :type "PrimitiveComponent Object Reference") (NormalImpulse :type "Vector Structure") (Hit :type "HitResult Structure (by ref)"))
  (bind _returnvalue (`KismetMathLibrary.VSize` NormalImpulse))
  (`/Engine/EditorBlueprintResources/StandardMacros.Gate` false :!label _label
    (:`Exit`
      (if (> _returnvalue 2000.0)
        (`|ExecutionSequence`
          (:`then_0`
            (goto _label :!via `Close`))
          (:`then_1`
            (`self.SmashEffect` (`.Location` (`GameplayStatics.BreakHitResult` Hit)))
            (`KismetSystemLibrary.PrintString` (`KismetTextLibrary.Conv_TextToString` (`|FormatText` "Physics Object Force: {force}" _returnvalue)) true true (struct :`R` 1.0 :`B` 0.589913 :`A` 1.0))
            (`KismetSystemLibrary.Delay` 0.2)
            (goto _label :!via `Open`)))))))

(event `SmashEffect`
  (params (Location :type "Vector Structure"))
  (`GameplayStatics.PlaySoundAtLocation` (select `/Game/Blueprints/Level_Items/ENUM_ImpactNoice` (`self.ImpactNoise`) :`NewEnumerator0` "/Game/Sounds/SFX/fart_impact/fart_impact.fart_impact" :`NewEnumerator1` "/Game/Sounds/SFX/metal_impact/metal_impact.metal_impact" :!type "SoundBase Object Reference") (`SceneComponent.K2_GetComponentLocation` (`self.Prop`)) (struct) 1.0 1.0 0.0 null null null null)
  (`NiagaraFunctionLibrary.SpawnSystemAtLocation` (select `/Game/Blueprints/Level_Items/ENUM_ImpactNoice` (`self.ImpactNoise`) :`NewEnumerator0` "/Game/Realistic_Starter_VFX_Pack_Niagara/Niagara/Explosion/fart.fart" :`NewEnumerator1` "/Game/Realistic_Starter_VFX_Pack_Niagara/Niagara/Destruction/metal.metal" :!type "NiagaraSystem Object Reference") Location)
  (`self.Smash`))

(fn `UserConstructionScript`
  (`StaticMeshComponent.SetStaticMesh` (`self.Prop`) (`self.StaticMesh`))
  (`PrimitiveComponent.SetMassOverrideInKg` (`self.Prop`) "None" (`self.ObjectMass`) true))