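; BP_FingerScanner is an interactable scanner that tries to start the player's shift, succeeding on roughly one in three scans.
; Success sets ShiftStarted on itself and on BP_GM, after which interaction does nothing.
; Failure starts a warm-up on a retriggerable delay, and interacting during it restarts the timer.
; Each outcome prints a debug message and plays its sound by swapping the clip on one Sound component.
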(event `/Game/Blueprints/Level_Items/BP_InteractInterface.Interact`
  (params (IsTired :type Boolean) (Character :type "/Game/Blueprints/BP_MainChar Object Reference"))
  (if (`self.bShiftStarted`)
    _
    (elif (`self.bWarmingUp`)
      (`KismetSystemLibrary.PrintString` "Warming Up")
      (`self.Warm Up`)
      (`self.PlaySound` "/Game/Sounds/Dialogue/scanner/scan_wait.scan_wait")
      (elif (> (`KismetMathLibrary.RandomIntegerInRange` 0 100) 66)
        (bind _asbp_gm (cast `/Game/Blueprints/BP_GM` (`GameplayStatics.GetGameMode`)))
        (set `/Game/Blueprints/BP_GM.bShiftStarted` true _asbp_gm)
        (`KismetSystemLibrary.PrintString` "ShiftStarted" true true (struct :`R` 0.120157 :`G` 1.0 :`A` 1.0))
        (set `self.bShiftStarted` true)
        (`self.PlaySound` "/Game/Sounds/Dialogue/scanner/scan_success.scan_success")
        (else
          (`KismetSystemLibrary.PrintString` "Shift did not start" true true (struct :`R` 1.0 :`B` 0.12254 :`A` 1.0))
          (`self.Warm Up`)
          (`self.PlaySound` "/Game/Sounds/Dialogue/scanner/scan_failed.scan_failed"))))))

(event `Warm Up`
  ;[1 1 1] Warm Up
  (set `self.bWarmingUp` true)
  (`KismetSystemLibrary.RetriggerableDelay` (`self.WarmUpDuration`))
  (set `self.bWarmingUp` false))

(event `PlaySound`
  (params (Sound :type "SoundBase Object Reference"))
  (bind _sound (`self.Sound`))
  (`AudioComponent.SetSound` _sound Sound)
  (`AudioComponent.Play` _sound 0.0))

(fn `UserConstructionScript`)