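; BP_Coffee is a physics coffee pickup that clears the interacting character's tire effect and meter, plays a sip sound and destroys itself.
; On BeginPlay it launches the Coffee component with a randomized impulse.
; Hard hits trigger a fart sound and particle effect plus a debug force printout, with a gate and short delay throttling repeats.
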(event `self.ReceiveBeginPlay`
  (bind _returnvalue (`KismetMathLibrary.RandomIntegerInRange` 0 3))
  (`PrimitiveComponent.AddImpulse` (`self.Coffee`) (`KismetMathLibrary.MakeVector` (select `int` _returnvalue :`0` (`KismetMathLibrary.RandomFloatInRange` 2500.0 10000.0) :`1` 0.0) (select `int` _returnvalue :`0` 0.0 :`1` (`KismetMathLibrary.RandomFloatInRange` 2500.0 10000.0)) (select `int` _returnvalue :`0` 0.0 :`1` 0.0 :`2` (`KismetMathLibrary.RandomFloatInRange` 2500.0 10000.0))) "None" false))

(event `/Game/Blueprints/Level_Items/BP_InteractInterface.Interact`
  (params (IsTired :type Boolean) (Character :type "/Game/Blueprints/BP_MainChar Object Reference"))
  (`/Engine/EditorBlueprintResources/StandardMacros.IsValid` Character
    (:`Is Valid`
      (`/Game/Blueprints/BP_MainChar.ClearTireEffect` Character)
      (set `/Game/Blueprints/BP_MainChar.TireMeter` 0 Character)
      (`GameplayStatics.PlaySound2D` "/Game/Sounds/SFX/sip/sip.sip" 1.0 1.0 0.0 null null)
      (`self.K2_DestroyActor`))))

(event `self.Coffee.OnComponentHit`
  (params (HitComponent :type "PrimitiveComponent Object Reference") (OtherActor :type "Actor Object Reference") (OtherComp :type "PrimitiveComponent Object Reference") (NormalImpulse :type "Vector Structure") (Hit :type "HitResult Structure (by ref)"))
  (bind _returnvalue (`KismetMathLibrary.VSize` NormalImpulse))
  (`/Engine/EditorBlueprintResources/StandardMacros.Gate` false :!label _label
    (:`Exit`
      (if (> _returnvalue 2000.0)
        (`|ExecutionSequence`
          (:`then_0`
            (goto _label :!via `Close`))
          (:`then_1`
            (`self.SmashEffect` (`.Location` (`GameplayStatics.BreakHitResult` Hit)))
            (`KismetSystemLibrary.PrintString` (`KismetTextLibrary.Conv_TextToString` (`|FormatText` "Physics Object Force: {force}" _returnvalue)) true true (struct :`R` 1.0 :`B` 0.589913 :`A` 1.0))
            (`KismetSystemLibrary.Delay` 0.2)
            (goto _label :!via `Open`)))))))

(event `SmashEffect`
  (params (Location :type "Vector Structure"))
  (`GameplayStatics.PlaySoundAtLocation` "/Game/Sounds/SFX/fart_impact/fart_impact.fart_impact" (`SceneComponent.K2_GetComponentLocation` (`self.Coffee`)) (struct) 1.0 1.0 0.0 null null null null)
  (`NiagaraFunctionLibrary.SpawnSystemAtLocation` "/Game/Realistic_Starter_VFX_Pack_Niagara/Niagara/Explosion/fart.fart" Location))

(fn `UserConstructionScript`)