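; BP_GM runs the day-shift clock, counting minutes late until the shift starts.
; Tick drives a short Delay that increments Time, converts it to hour and minute, debug-prints it and calls a clock tick.
; A Gate fires a random email or meeting call once at minutes 30 and 59.
; From hour 17, a DoOnce teleports the player and shows the end screen.
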(event `Timer`
  ;[1 1 1] Day Shift Timer
  ;[1 1 1] Should be quicker than real life (4 min atm)
  (`KismetSystemLibrary.Delay` 0.008334)
  (if (and (`self.bTimerOn`) (`self.bShiftStarted`))
    (bind _result (`/Engine/EditorBlueprintResources/StandardMacros.IncrementFloat` (`self.Time`))
      (:`  `
        (set `self.Hour` (`KismetMathLibrary.FFloor` (mod (/ _result 3600.0) 24.0)))
        (set `self.Minute` (`KismetMathLibrary.FFloor` (mod (/ _result 60.0) 60.0)))
        (`|ExecutionSequence`
          (:`then_0`
            (`KismetSystemLibrary.PrintString` (`KismetTextLibrary.Conv_TextToString` (`|FormatText` "{hour}:{second}" (`self.Hour`) (`self.Minute`))) true true (struct :`R` 0.046721 :`G` 1.0 :`B` 0.002988 :`A` 1.0) 0.1 "0"))
          (:`then_2`
            (`self.Check for PC notifications`))
          (:`then_3`
            (`self.CheckForEndOfDay`))
          (:`then_4`
            (`self.ClockTick`)))))
    (elif (not (`self.bShiftStarted`))
      (`/Engine/EditorBlueprintResources/StandardMacros.IncrementInt` (`self.MinutesLate`)))))

(event `self.ReceiveTick`
  (params (DeltaSeconds :type "Float (single-precision)"))
  ;[1 1 1] Tick
  (`|ExecutionSequence`
    (:`then_0`
      (`self.Timer`))))

(event `Check for PC notifications`
  (bind _minute (`self.Minute`))
  ;[1 1 1] Check for pc notification
  (if (or (== _minute 30) (== _minute 59))
    (`/Engine/EditorBlueprintResources/StandardMacros.Gate` false :!label _label
      (:`Exit`
        (`|ExecutionSequence`
          (:`then_0`
            (goto _label :!via `Close`))
          (:`then_1`
            (if (> (`KismetMathLibrary.RandomIntegerInRange` 0 100) 50)
              (`self.NewEmail`)
              (else
                (`self.NewMeeting`)))))))
    (else
      (goto _label :!via `Open`))))

(event `self.ReceiveBeginPlay`
  ;[1 1 1] Begin Play
  (`|ExecutionSequence`
    (:`then_0`
      (`self.GetGameInstance`))
    (:`then_1`
      (`self.OnDayStarted`))))

(event `GetGameInstance`
  ;[1 1 1] Get G Instance
  (bind _asbp_game_instance (cast `/Game/Blueprints/BP_GameInstance` (`GameplayStatics.GetGameInstance`)))
  (set `self.As BP Game Instance` _asbp_game_instance))

(event `CheckForEndOfDay`
  (if (>= (`self.Hour`) 17)
    (`/Engine/EditorBlueprintResources/StandardMacros.DoOnce` false
      (:`Completed`
        (`self.K2_SetActorLocation` (`GameplayStatics.GetPlayerCharacter` 0) (278.0 -5361.0 158.0) false true)
        (bind _returnvalue (`|CreateWidget` "/Game/Blueprints/Widgets/Widget_EndScreen.Widget_EndScreen_C"))
        (`UserWidget.AddToViewport` _returnvalue 0)))))

(event `OnDayStarted`
  ;[1 1 1] On Day Started
  (`/Engine/EditorBlueprintResources/StandardMacros.IsValid` (`self.As BP Game Instance`)
    (:`Is Valid`
      (`KismetSystemLibrary.PrintString` (`KismetStringLibrary.Conv_IntToString` (`/Game/Blueprints/BP_GameInstance.CurrentDay` (`self.As BP Game Instance`)))))))

(fn `UserConstructionScript`)